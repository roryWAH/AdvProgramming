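; PC_LocalMult is a player controller that, as its name suggests, serves local multiplayer and lets its player join the game on input.
; On BeginPlay it waits briefly, then adds the default Enhanced Input mapping context to its local player subsystem, if valid.
; The join action asks the game mode to restart the player, spawning a pawn only when the controller has none.
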(event Input|EnhancedActionEvents|EnhancedInputActionIA_Join_Game
  (params (ActionValue :type Boolean) (ElapsedSeconds :type Float%20%28double-precision%29) (TriggeredSeconds :type Float%20%28double-precision%29) (InputAction :type Input%20Action%20Object%20Reference :default "/Game/ThirdPerson/Input/Actions/IA_Join_Game.IA_Join_Game"))
  (Utilities|IsValid (Pawn|GetControlledPawn)
    (:Is%20Not%20Valid
      (Class|GameModeBase|RestartPlayer (Game|GetGameMode) self))))

(event EventBeginPlay
  (bind _self self)
  (bind _returnvalue (PlayerController|LocalPlayerSubsystems|GetEnhancedInputLocalPlayerSubsystem _self))
  (Utilities|FlowControl|Delay 0.2)
  (Utilities|IsValid _returnvalue
    (:Is%20Valid
      (Input|AddMappingContext _returnvalue "/Game/ThirdPerson/Input/IMC_Default.IMC_Default" 0 "(bIgnoreAllPressedKeysUntilRelease=True,bForceImmediately=False,bNotifyUserSettings=False)"))))

(event EventTick
  (params (DeltaSeconds :type Float%20%28single-precision%29)))

(fn ConstructionScript)